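; TargetRunner's player state, tracking targets hit and destroyed, current and high score, unlocked tools and level progress.
; Energy and Animus live in attribute components, with functions to add or deduct energy, add or reset Animus and pause its recharge.
; It converts its state to and from a save data struct, though ammo, goods and hit-count maps are saved empty.
; It also builds level run stats from the game mode seed and game state level number.
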(event `OnTargetHit`
  (params (Score :type "Float (double-precision)") (TargetDestroyed :type Boolean))
  ;[1 1 1] Handles targets hit and score.
  (`|ExecutionSequence`
    (:`then_0`
      (`/Engine/EditorBlueprintResources/StandardMacros.IncrementInt` (`self.TargetsHit`)
        (:`  `
          (`/Engine/EditorBlueprintResources/StandardMacros.IncrementInt` (`self.TotalTargetsHit`)))))
    (:`then_1`
      (if TargetDestroyed
        (`/Engine/EditorBlueprintResources/StandardMacros.IncrementInt` (`self.TargetsDestroyed`)
          (:`  `
            (`/Engine/EditorBlueprintResources/StandardMacros.IncrementInt` (`self.TotalTargetsDestroyed`))))))
    (:`then_2`
      (bind _output_get (set `self.CurrentScore` (+ Score (`self.CurrentScore`))))
      (if (> _output_get (`self.HighScore`))
        (set `self.HighScore` (`self.CurrentScore`))))))

(event `UpdateFromSaveData`
  (params (PlayerSaveData :type "PlayerSaveData Structure"))
  (bind (_name _displayname _maxlevelcompleted _totalrunsplayed _totalplaytimeinruns _resourceonetotal _resourcetwototal _targetshit _currentscore _totaltargetshit _highscore _maxhealth _maxenergy _targetsdestroyed _totaltargetsdestroyed _energyregenrate _resourceonespent _resourcetwospent _toolsunlocked) (break `PlayerSaveData` PlayerSaveData))
  (`|ExecutionSequence`
    (:`then_0`
      (set `self.MaxLevelCompleted` _maxlevelcompleted))
    (:`then_1`
      (set `self.TargetsHit` (`KismetMathLibrary.FTrunc` _targetshit)))
    (:`then_2`
      (set `self.CurrentScore` _currentscore))
    (:`then_3`
      (set `self.TotalTargetsHit` (`KismetMathLibrary.FTrunc` _totaltargetshit)))
    (:`then_4`
      (set `self.HighScore` _highscore))
    (:`then_5`
      (set `self.MaxHealth` _maxhealth))
    (:`then_6`
      (set `TR_ActorAttributeComponent.MaxValue` _maxenergy (`self.EnergyAttrComponent`)))
    (:`then_7`
      (set `self.TargetsDestroyed` (`KismetMathLibrary.FTrunc` _targetsdestroyed)))
    (:`then_8`
      (set `self.TotalTargetsDestroyed` (`KismetMathLibrary.FTrunc` _totaltargetsdestroyed)))
    (:`then_9`
      (set `TR_ActorAttributeComponent.RechargeRate` _energyregenrate (`self.EnergyAttrComponent`)))
    (:`then_10`
      (if true
        (set `self.ToolsUnlocked` _toolsunlocked)))))

(event `UnlockTool`
  (params (ToolName :type Name))
  (`KismetArrayLibrary.Array_AddUnique` (`self.ToolsUnlocked`) ToolName))

(event `PauseAnimus`
  (set `TR_ActorAttributeComponent.bRechargePaused` true (`self.AnimusAttrComponent`)))

(event `ResumeAnimus`
  (set `TR_ActorAttributeComponent.bRechargePaused` false (`self.AnimusAttrComponent`)))

(event `ResetAnimus`
  (`TR_ActorAttributeComponent.ResetToMax` (`self.AnimusAttrComponent`)))

(fn `AddAnimus`
  (params (ToAdd :type "Float (double-precision)"))
  (returns (CurrentAnimus :type "Float (double-precision)"))
  (bind _animusattrcomponent (`self.AnimusAttrComponent`))
  (`TR_ActorAttributeComponent.DeltaValue` _animusattrcomponent ToAdd true)
  (return (`TR_ActorAttributeComponent.CurrentValue` _animusattrcomponent)))

(fn `AddEnergy`
  (params (ToAdd :type "Float (double-precision)"))
  (returns (CurrentEnergy :type "Float (double-precision)"))
  (bind _energyattrcomponent (`self.EnergyAttrComponent`))
  (`TR_ActorAttributeComponent.DeltaValue` _energyattrcomponent ToAdd true)
  (return (`TR_ActorAttributeComponent.CurrentValue` _energyattrcomponent)))

(fn `DeductEnergy`
  (params (ToDeduct :type "Float (double-precision)"))
  (returns (Successful :type Boolean) (Remaining :type "Float (double-precision)"))
  (bind _energyattrcomponent (`self.EnergyAttrComponent`))
  (bind _returnvalue (`TR_ActorAttributeComponent.DeltaValue` _energyattrcomponent (* ToDeduct -1.0) false))
  (return _returnvalue (`TR_ActorAttributeComponent.CurrentValue` _energyattrcomponent)))

(fn `GetCurrentEnergy`
  (returns (CurrentEnergy :type "Float (double-precision)"))
  (return (`TR_ActorAttributeComponent.CurrentValue` (`self.EnergyAttrComponent`))))

(fn `GetLevelRunStats`
  (returns (LevelRunStats :type "LevelRunStats Structure"))
  (bind _astr_game_mode_base_bp (cast `/Game/TargetRunner/Blueprints/Game/TR_GameMode_Base_BP` (`GameplayStatics.GetGameMode`)))
  (bind _astr_game_state_bp (cast `/Game/TargetRunner/Blueprints/Game/TR_GameState_BP` (`GameplayStatics.GetGameState`)))
  (return (make `LevelRunStats` false (`TR_GameState.CurrentLevelNumber` _astr_game_state_bp) (`self.CurrentScore`) (`GameplayStatics.GetUnpausedTimeSeconds`) (`KismetMathLibrary.Conv_IntToDouble` (`/Game/TargetRunner/Blueprints/Game/TR_GameMode_Base_BP.GeneratorSeed` _astr_game_mode_base_bp)) (`|MakeArray`))))

(fn `GetPlayerSaveData`
  (returns (PlayerSaveData :type "PlayerSaveData Structure"))
  (bind _playername (`self.PlayerName`))
  (return (make `PlayerSaveData` (`KismetStringLibrary.Conv_StringToName` (`KismetTextLibrary.Conv_TextToString` _playername)) _playername (`self.MaxLevelCompleted`) 0.0 0.0 0.0 0.0 (`KismetMathLibrary.Conv_IntToDouble` (`self.TargetsHit`)) (`self.CurrentScore`) (`KismetMathLibrary.Conv_IntToDouble` (`self.TotalTargetsHit`)) (`self.HighScore`) (`self.MaxHealth`) (`TR_ActorAttributeComponent.MaxValue` (`self.EnergyAttrComponent`)) (`KismetMathLibrary.Conv_IntToDouble` (`self.TargetsDestroyed`)) (`KismetMathLibrary.Conv_IntToDouble` (`self.TotalTargetsDestroyed`)) (`TR_ActorAttributeComponent.RechargeRate` (`self.EnergyAttrComponent`)) 0.0 0.0 (`self.ToolsUnlocked`) (`|MakeMap`) (`|MakeMap`) (`|MakeMap`))))

(fn `UserConstructionScript`)